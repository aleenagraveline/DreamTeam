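; BasicEnemy is a simple enemy actor that lunges at the player's third-person character when it overlaps that character.
; On overlap, MoveComponentTo slides the root over one second to a point slightly past the player's position at that moment, horizontally, without further tracking.
; Ending the overlap clears SeesPlayer, which this graph never reads or sets true.
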(event EventBeginPlay)

(event Collision|EventActorBeginOverlap
  (params (OtherActor :type Actor%20Object%20Reference))
  (bind _asbp_third_person_character (Utilities|Casting|CastToBP_ThirdPersonCharacter OtherActor))
  (Components|MoveComponentTo (Variables|Default|GetDefaultSceneRoot) (+ (Transformation|GetActorLocation _asbp_third_person_character) (* (Math|Vector|Normalize (- (Transformation|GetActorLocation _asbp_third_person_character) (Transformation|GetActorLocation))) "10.000000,10.000000,0.000000")) "0, 0, 0" false false 1.0 false))

(event Collision|EventActorEndOverlap
  (params (OtherActor :type Actor%20Object%20Reference))
  (Utilities|Casting|CastToBP_ThirdPersonCharacter OtherActor)
  (Variables|Default|SetSeesPlayer false))

(fn ConstructionScript)