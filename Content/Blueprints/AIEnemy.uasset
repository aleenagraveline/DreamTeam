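; AI enemy character that chases the third-person player, damages them on contact and can be damaged and destroyed.
; PawnSensing sets the target and issues AIMoveTo while following is allowed.
; Tick uses a visibility line trace and distance check to allow following, or halt movement when either fails.
; Incoming damage reduces health, with a brief delay-based invincibility window that callers can bypass.
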(event OnSeePawn(PawnSensing)
  (params (Pawn :type Pawn%20Object%20Reference))
  ;[0.08933 0.571 1] Follow Player
  (bind _asbp_third_person_character (Utilities|Casting|CastToBP_ThirdPersonCharacter Pawn))
  (Variables|Default|SetTargetPlayer _asbp_third_person_character)
  (if (Variables|Default|GetCanFollowPlayer)
    (AI|AIMoveTo self (.RandomLocation (AI|Navigation|GetRandomReachablePointinRadius (Transformation|GetWorldLocation (Variables|/Script/Engine.Actor|GetRootComponent _asbp_third_person_character)) 1.0 0 0)) _asbp_third_person_character 1.0 false)))

(event Custom|DamageEnemy
  (params (IgnoreIFrames :type Boolean) (DmgAmount :type Integer))
  (if IgnoreIFrames
    (if (<= (- (Variables|Default|GetEnemyHealth) DmgAmount) 0) :!label _label
      (Actor|DestroyActor)
      (else
        (Variables|Default|SetEnemyHealth (- (Variables|Default|GetEnemyHealth) DmgAmount))
        (Variables|Default|SetHasIFrames true)
        (Utilities|FlowControl|Delay 0.5)
        (Variables|Default|SetHasIFrames false)))
    (elif (Variables|Default|GetHasIFrames)
      (Development|PrintString "(I Frames Enemy)")
      (else
        (goto _label)))))

(event EventTick
  (params (DeltaSeconds :type Float%20%28single-precision%29))
  (bind _targetplayer (Variables|Default|GetTargetPlayer))
  ;[1 0.05104 0.05104] Stop/disable follow if player is not visible and within targeting distance
  (Variables|Default|GetTargetPlayer
    (:then
      (bind _outhit (Collision|LineTraceByChannel (Transformation|GetActorLocation) (Transformation|GetActorLocation _targetplayer) "TraceTypeQuery1" false 0 "None"))
      (if (and (== (|HitActor _outhit) _targetplayer) (<= (Transformation|GetDistanceTo _targetplayer) (Variables|Default|GetMaxTargetingDist)))
        (Variables|Default|SetCanFollowPlayer true)
        (else
          (Components|Movement|StopMovementImmediately (Variables|Character|GetCharacterMovement))
          (Variables|Default|SetCanFollowPlayer false))))
    (:else)))

(fn ConstructionScript)

(event Collision|EventHit
  (params (MyComp :type Primitive%20Component%20Object%20Reference) (Other :type Actor%20Object%20Reference) (OtherComp :type Primitive%20Component%20Object%20Reference) (bSelfMoved :type Boolean) (HitLocation :type Vector :default "0, 0, 0") (HitNormal :type Vector :default "0, 0, 0") (NormalImpulse :type Vector :default "0, 0, 0") (Hit :type Hit%20Result%20Structure%20%28by%20ref%29))
  (return (.hitactor Hit)))