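; Trigger actor that flips the third-person character's camera when the player passes into it.
; On begin overlap it stores the character's YDirection as the entrance direction and calls FlipCamera on the character.
; On end overlap it compares the current YDirection with the stored one and flips the camera again if the player swapped direction inside the trigger.
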(event Collision|EventActorBeginOverlap
  (params (OtherActor :type Actor%20Object%20Reference))
  ;[0.2547 1 0.1689] Flip Camera & Store Direction Of Player When Entering Trigger
  (bind _asbp_third_person_character (Utilities|Casting|CastToBP_ThirdPersonCharacter OtherActor))
  (Variables|Default|SetEntranceDirection (Variables|/Game/ThirdPerson/Blueprints/BP_ThirdPersonCharacter.BP_ThirdPersonCharacter_C|GetYDirection _asbp_third_person_character))
  (Default|FlipCamera _asbp_third_person_character))

(event Collision|EventActorEndOverlap
  (params (OtherActor :type Actor%20Object%20Reference))
  ;[1 0.05521 0.05521] Check If Player Swapped Directions While In Trigger & Flip Camera Again If Necessary
  (bind _asbp_third_person_character (Utilities|Casting|CastToBP_ThirdPersonCharacter OtherActor))
  (if (!= (Variables|/Game/ThirdPerson/Blueprints/BP_ThirdPersonCharacter.BP_ThirdPersonCharacter_C|GetYDirection _asbp_third_person_character) (Variables|Default|GetEntranceDirection))
    (Default|FlipCamera _asbp_third_person_character)))

(fn ConstructionScript)